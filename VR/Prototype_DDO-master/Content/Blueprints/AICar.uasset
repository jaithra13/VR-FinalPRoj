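; AICar is a traffic car actor that drives straight ahead and turns into a physics object when the player hits it.
; The construction script picks a random mesh from CarModels.
; Tick moves the actor along its forward vector by a fixed, frame-rate-dependent step without sweeping.
; Overlap with an actor whose display name is "PlayerPawn" enables mesh physics, then destroys the car after a delay.
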(event EventBeginPlay)

(event Collision|EventActorBeginOverlap
  (params (OtherActor :type Actor%20Object%20Reference))
  ;[0 0 0] Enable physics when colliding with the player
  (if (Utilities|Enum|Equal(Enum) (Utilities|GetDisplayName OtherActor) "PlayerPawn")
    (Physics|SetSimulatePhysics (Variables|Default|GetStaticMesh) true)
    (Utilities|FlowControl|Delay 9.0)
    (Actor|DestroyActor)))

(event EventTick
  (params (DeltaSeconds :type Float%20%28single-precision%29))
  (Transformation|SetActorLocation (+ (Transformation|GetActorLocation) (* (Transformation|GetActorForwardVector) 2e+01)) false false))

(fn ConstructionScript
  (bind _carmodels (Variables|Default|GetCarModels))
  (Components|StaticMesh|SetStaticMesh (Variables|Default|GetStaticMesh) (Utilities|Array|Get(acopy) _carmodels (Math|Random|RandomInteger (Utilities|Array|Length _carmodels)))))