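; LapViewPawn is a possessable pawn for a sandwich-building minigame, showing the mouse cursor while possessed.
; GrabItem toggles a physics-handle hold on CanGrab components found by a cursor trace, following the deprojected mouse ray with wheel-adjusted distance.
; MoveRight input applies sideways force to the pawn's own CanGrab meshes.
; SandwichTrigger overlaps advance a counter when ingredient tags match IngredientsOrder, showing the win screen after five.
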(event OnComponentBeginOverlap(SandwichTrigger)
  (params (OverlappedComponent :type Primitive%20Component%20Object%20Reference) (OtherActor :type Actor%20Object%20Reference) (OtherComp :type Primitive%20Component%20Object%20Reference) (OtherBodyIndex :type Integer) (bFromSweep :type Boolean) (SweepResult :type Hit%20Result%20Structure%20%28by%20ref%29))
  (if (!= (Variables|Default|GetIngredientCounter) 5)
    (if (Utilities|Array|ContainsItem (Variables|/Script/Engine.ActorComponent|GetComponentTags OtherComp) (Utilities|String|StringToName (Utilities|Array|Get(acopy) (Variables|Default|GetIngredientsOrder) (Variables|Default|GetIngredientCounter))))
      (bind _result (Math|Integer|IncrementInt (Variables|Default|GetIngredientCounter))
        (:%20%20
          (if (== _result 5)
            (bind _returnvalue (UserInterface|CreateWidget "/Game/Blueprints/PauseMenu/WinScreenWidget.WinScreenWidget_C" (Game|GetPlayerController 0)))
            (UserInterface|Viewport|AddtoViewport _returnvalue 0)))))))

(event EventBeginPlay)

(event EventTick
  (params (DeltaSeconds :type Float%20%28single-precision%29))
  (bind _returnvalue (Game|GetPlayerController 0))
  (bind (_worldlocation _worlddirection) (Game|Player|ConvertMouseLocationToWorldSpace _returnvalue))
  (Utilities|IsValid (Variables|Default|GetHeldObject)
    (:Is%20Valid
      (Physics|Components|PhysicsHandle|SetTargetLocation (Variables|Default|GetPhysicsHandle) (+ _worldlocation (* _worlddirection (- (Variables|Default|GetOriginalObjectDistance) (Variables|Default|GetDistanceModifier))))))))

(event EventPossessed
  (params (NewController :type Controller%20Object%20Reference))
  (bind _asplayer_controller (Utilities|Casting|CastToPlayerController NewController))
  (Variables|/Script/Engine.PlayerController|SetbShowMouseCursor _asplayer_controller true))

(event EventUnpossessed
  (params (OldController :type Controller%20Object%20Reference))
  (CallFunction|DropItem)
  (bind _asplayer_controller (Utilities|Casting|CastToPlayerController OldController))
  (Variables|/Script/Engine.PlayerController|SetbShowMouseCursor _asplayer_controller false))

(event Input|ActionEvents|InputActionGrabItem
  (params (Key :type Key%20Structure :default "None"))
  (:Pressed
    (Utilities|IsValid (Variables|Default|GetHeldObject)
      (:Is%20Valid
        (CallFunction|DropItem))
      (:Is%20Not%20Valid
        (bind (_hit _hitresult) (CallFunction|LineTrace))
        (if (and _hit (Utilities|Array|ContainsItem (Variables|/Script/Engine.ActorComponent|GetComponentTags (.HitComponent (Collision|BreakHitResult _hitresult))) "CanGrab"))
          (CallFunction|GrabItem _hitresult))))))

(event Input|AxisEvents|InputAxisMoveRight
  (params (AxisValue :type Float%20%28single-precision%29))
  (if (!= AxisValue 0.0)
    (for _array_element (Actor|GetComponentsbyTag "/Script/Engine.StaticMeshComponent" "CanGrab")
      (if (< AxisValue 0.0)
        (Physics|AddForce _array_element "0,300.000000, 0" "None" false)
        (else
          (Physics|AddForce _array_element "0,-300.000000, 0" "None" false))))))

(event Input|MouseEvents|MouseWheelDown
  (params (Key :type Key%20Structure :default "None"))
  (:Pressed
    (Variables|Default|SetDistanceModifier (Math|Float|Clamp(Float) (+ (Variables|Default|GetDistanceModifier) 2.0) 0.0 5e+01))))

(event Input|MouseEvents|MouseWheelUp
  (params (Key :type Key%20Structure :default "None"))
  (:Pressed
    (Variables|Default|SetDistanceModifier (Math|Float|Clamp(Float) (- (Variables|Default|GetDistanceModifier) 2.0) 0.0 5e+01))))

(fn ConstructionScript)

(fn GrabItem
  (params (Hit%20Result :type Hit%20Result%20Structure))
  (bind (_bblockinghit _binitialoverlap _time _distance _location _impactpoint _normal _impactnormal _physmat _hitactor _hitcomponent) (Collision|BreakHitResult Hit%20Result))
  (bind _output_get (Variables|Default|SetHeldObject _hitcomponent))
  (Variables|Default|SetOriginalObjectDistance _distance)
  (Physics|Components|PhysicsHandle|GrabComponentatLocationwithRotation (Variables|Default|GetPhysicsHandle) (Variables|Default|GetHeldObject) "None" (Transformation|GetWorldLocation _output_get) "0, 0, 0"))

(fn DropItem
  (Physics|Components|PhysicsHandle|ReleaseComponent (Variables|Default|GetPhysicsHandle))
  (Variables|Default|SetHeldObject 0))

(fn LineTrace
  (bind _returnvalue (Game|GetPlayerController 0))
  (bind (_worldlocation _worlddirection) (Game|Player|ConvertMouseLocationToWorldSpace _returnvalue))
  (bind (_outhit _returnvalue_2) (Collision|LineTraceByChannel (Transformation|GetWorldLocation (Variables|Default|GetCamera)) (+ _worldlocation (* _worlddirection 1e+04)) "TraceTypeQuery1" false 0 "None" false))
  (return _returnvalue_2 _outhit))