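; Road segment actor for an endlessly generated road, randomly dressed with scenery.
; Construction caches three AI spawn point transforms, jitters the tree's position and yaw, randomly swaps its mesh, and randomly adds houses at two spawn points.
; When PlayerPawn overlaps it, it asks PrototypeGameMode for a new road, spawns a car on that road if CanSpawnAI allows, clears the flag, then destroys itself after a short delay.
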(event EventBeginPlay)

(event Collision|EventActorBeginOverlap
  (params (OtherActor :type Actor%20Object%20Reference))
  ;[0 0 0] When the player reaches the end of the road, spawn a new one and destroy the current road
  (Utilities|Casting|CastToPlayerPawn OtherActor)
  (bind _asprototype_game_mode (Utilities|Casting|CastToPrototypeGameMode (Game|GetGameMode)))
  (bind _road (Default|SpawnRoad _asprototype_game_mode))
  (if (Variables|/Game/Blueprints/PrototypeGameMode.PrototypeGameMode_C|GetCanSpawnAI _asprototype_game_mode)
    (Default|SpawnCar _asprototype_game_mode (Variables|RoadPrefab_C|GetSpawnPoints _road))
    (Variables|/Game/Blueprints/PrototypeGameMode.PrototypeGameMode_C|SetCanSpawnAI _asprototype_game_mode false))
  (Utilities|FlowControl|Delay 2.0)
  (Actor|DestroyActor))

(fn ConstructionScript
  (CallFunction|SetAISpawnPoints)
  (CallFunction|RandomTransform (Variables|Default|GetTree))
  (CallFunction|RandomTreeMesh)
  (CallFunction|SpawnHouses))

(fn GetAttachTransform
  (return (Transformation|GetWorldTransform (Variables|Default|GetAttachPoint))))

(fn SetAISpawnPoints
  (Variables|Default|SetSpawnPoints (Utilities|Array|MakeArray (Transformation|GetWorldTransform (Variables|Default|GetAISpawnPoint1)) (Transformation|GetWorldTransform (Variables|Default|GetAISpawnPoint2)) (Transformation|GetWorldTransform (Variables|Default|GetAISpawnPoint3)))))

(fn SpawnAI)

(fn RandomTransform
  (params (Object :type Static%20Mesh%20Component%20Object%20Reference))
  (bind _relativerotation (Variables|/Script/Engine.SceneComponent|GetRelativeRotation Object))
  (bind _relativelocation (Variables|/Script/Engine.SceneComponent|GetRelativeLocation Object))
  (bind (_x _y _z) (Math|Vector|BreakVector _relativelocation))
  (bind (_roll _pitch _yaw) (Math|Rotator|BreakRotator _relativerotation))
  (Transformation|SetRelativeLocationAndRotation Object (Math|Vector|MakeVector (+ _x (Math|Random|RandomFloatinRange -75.0 75.0)) (+ _y (Math|Random|RandomFloatinRange -75.0 75.0)) _z) (Math|Rotator|MakeRotator _roll _pitch (+ _yaw (Math|Random|RandomFloatinRange 0.0 9e+01))) false false))

(fn RandomTreeMesh
  (if (== (Math|Random|RandomInteger 2) 1)
    (Components|StaticMesh|SetStaticMesh (Variables|Default|GetTree) "/Game/Models/Buildings_etc/Tree2.Tree2")))

(fn SpawnHouses
  (Utilities|FlowControl|Sequence
    (:then_0
      (if (>= (Math|Random|RandomInteger 10) 3)
        (AddComponent|AddChildActorComponent false (Math|Transform|MakeTransform (.Location (Math|Transform|BreakTransform (Transformation|GetRelativeTransform (Variables|Default|GetHouseSpawnPoint)))) "0,90.000000, 0" "10.000000,10.000000,10.000000"))))
    (:then_1
      (if (>= (Math|Random|RandomInteger 10) 3)
        (AddComponent|AddChildActorComponent false (Math|Transform|MakeTransform (.Location (Math|Transform|BreakTransform (Transformation|GetRelativeTransform (Variables|Default|GetHouseSpawnPoint2)))) "0,-90.000000, 0" "10.000000,10.000000,10.000000"))))))